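; Base interactive activator with a floating, spinning mesh and player-proximity outline, which plays a sound and triggers linked popup actors.
; Remote interaction alternately raises and lowers it via timeline, locking input while rising.
; Collision mode hides the mesh for a Niagara glyph and fires on overlap, while Hold also fires on exit.
; Overlaps are filtered by component to the Light/Dark character capsules from BP_Manager, assigned carry items, or both.
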(event `self.ReceiveBeginPlay`
  ;[1 1 1] BeginPlay
  (`|ExecutionSequence`
    (:`then_0`
      (bind _returnvalue (`GameplayStatics.GetActorOfClass` "/Game/CoreMechanics/BP_Manager.BP_Manager_C"))
      (set `self.BP Manager` _returnvalue)
      (`self.Float`)
      (`self.Rotate`))
    (:`then_1`
      ;[0.005891 0.1406 0] If Hold is enabled, then automatically enable activision via collision and reverse. Collision and reverse are neceessary for Hold to work correctly.
      (if (`self.Activate (Hold)`)
        (set `self.Activate (On Collision)` true)))
    (:`then_2`
      ;[0.005891 0.1406 0] Is the activator set to be collision based? If so we need to hide the remote activator object and show the glyph
      (if (or (`self.Activate (On Collision)`) (`self.Activate (Hold)`))
        ;[0.005891 0.1406 0] If the activator is suppose to be a glyph (collision based) then
        (`SceneComponent.SetHiddenInGame` (`self.Activator Mesh`) true false)
        (`PrimitiveComponent.SetCollisionEnabled` (`self.Activator Mesh`) "NoCollision")
        (`ActorComponent.Activate` (`self.NS Base`) false)))))

(event `Rise`
  ;[1 1 1] Rise
  ;[0 0 0] This controls the code going up and down when activated and triggering the activation event
  ;;[0.005891 0.1406 0] Get the starting and end point of where we are transitioning to and from
  (bind _output_get (set `self.Activation Mesh Start Pos` (`SceneComponent.K2_GetComponentLocation` (`self.Activator Move Point`))))
  (set `self.Rise New Pos` (`KismetMathLibrary.MakeVector` (.x _output_get) (.y _output_get) (+ (.z _output_get) (`self.Rise Amount`))))
  ;;[0.005891 0.1406 0] Activate the visual feedback and play the code BEFORE moving the object
  (`ActorComponent.Activate` (`self.NS Activator`) false)
  (`self.Triggered Event`)
  ;;[0.005891 0.1406 0] Move the mesh upwards after activating visual feedback, or downwards from the reverse pin if it is called
  (bind (_direction _time) (`Timeline|Rise Mesh` :!via `PlayFromStart` :!label _label)
    (:`Update`
      (`SceneComponent.K2_SetWorldLocation` (`self.Activator Move Point`) (`KismetMathLibrary.VLerp` (`self.Activation Mesh Start Pos`) (`self.Rise New Pos`) _time) false false))
    (:`Finished`
      ;;[0.005891 0.1406 0] This bool controls if the player can or cannot interact with this object, it is turned off while moving and back on after it has finished moving
      (set `self.Is Interactable?` true))))

(event `Reverse Rise`
  ;[0 0 0] This controls the code going up and down when activated and triggering the activation event
  ;;[1 1 1] Reverse
  ;;[0.005891 0.1406 0] Activate the visual feedback and play the code BEFORE moving the object
  (`ActorComponent.Activate` (`self.NS Activator`) false)
  (`self.Triggered Event`)
  (goto _label :!via `Reverse`))

(event `self.OnInteract`
  (params (InteractingPlayer :type "/Game/ThirdPerson/Blueprints/BP_Player_Character Object Reference"))
  ;[1 1 1] Remote Code
  ;[0 0 0] Controls if the popup mechanic works via interface or not
  ;;[0.005891 0.1406 0] Checks to see if this activator can be used more than once
  (if (and (`self.Activate (Remotely)`) (`self.Is Interactable?`))
    (set `self.Is Interactable?` false)
    (`/Engine/EditorBlueprintResources/StandardMacros.FlipFlop`
      (:`A`
        (`self.Rise`))
      (:`B`
        (`self.Reverse Rise`)))))

(event `Float`
  ;[1 1 1] Float
  ;[0 0 0] Mesh bobs up and down in air
  ;;[0.005891 0.1406 0] Float up and down based on a VECTOR timeline instead of a float timeline
  (bind (_direction _newtrack_0) (`Timeline|Floating`)
    (:`Update`
      (`SceneComponent.K2_SetRelativeLocation` (`self.Activator Mesh`) _newtrack_0 false false))))

(event `self.Collision Box.OnComponentBeginOverlap`
  (params (OverlappedComponent :type "PrimitiveComponent Object Reference") (OtherActor :type "Actor Object Reference") (OtherComp :type "PrimitiveComponent Object Reference") (OtherBodyIndex :type Integer) (bFromSweep :type Boolean) (SweepResult :type "HitResult Structure (by ref)"))
  ;[1 1 1] Collision Code
  ;[0 0 0] Interaction Via Collision
  ;;[0.005891 0.1406 0] Is activation via collision enabled?
  (if (`self.Activate (On Collision)`)
    ;;[0.005891 0.1406 0] Is the actor that entered the collision box the player?
    (`self.What Can Activate Me?` OtherComp)
    (if (`self.Verified Actor`)
      (`ActorComponent.Activate` (`self.NS Active`) false)
      ;;[0.005891 0.1406 0] Run the code to trigger event
      (`self.Triggered Event`))))

(event `Rotate`
  (bind (_activation_mesh_start_rot_roll _activation_mesh_start_rot_pitch _activation_mesh_start_rot_yaw) (`KismetMathLibrary.BreakRotator` (`self.Activation Mesh Start Rot`)))
  ;[1 1 1] Rotate
  ;[0 0 0] Rotate the mesh actor in a slow and steady pace
  ;;[0.005891 0.1406 0] Get references for where the rotation starts and ends so we know what way we want to rotate
  (set `self.Activation Mesh Start Rot` (`SceneComponent.K2_GetComponentRotation` (`self.Activator Mesh`)))
  (set `self.Activation New Rot` (`KismetMathLibrary.MakeRotator` _activation_mesh_start_rot_roll _activation_mesh_start_rot_pitch (+ _activation_mesh_start_rot_yaw (`self.Rotate Amount`))))
  ;;[0.005891 0.1406 0] Rotate the object 360 degrees and once it is finished call the rotate code again to create a loop effect
  (bind (_direction _time) (`Timeline|Rotate Mesh` :!via `PlayFromStart`)
    (:`Update`
      (`SceneComponent.K2_SetWorldRotation` (`self.Activator Mesh`) (`KismetMathLibrary.RLerp` (`self.Activation Mesh Start Rot`) (`self.Activation New Rot`) _time) false false))
    (:`Finished`
      (`self.Rotate`))))

(event `self.Collision Box.OnComponentEndOverlap`
  (params (OverlappedComponent :type "PrimitiveComponent Object Reference") (OtherActor :type "Actor Object Reference") (OtherComp :type "PrimitiveComponent Object Reference") (OtherBodyIndex :type Integer))
  ;[1 1 1] Hold Code
  ;[0 0 0] Interaction Via Hold
  ;;[0.005891 0.1406 0] Is activation via collision enabled?
  (if (`self.Activate (Hold)`)
    ;;[0.005891 0.1406 0] Is the actor that entered the collision box the player?
    (`self.What Can Activate Me?` OtherComp)
    (if (`self.Verified Actor`)
      ;;[0.005891 0.1406 0] Run the code to trigger event
      (`self.Triggered Event`)
      (`ActorComponent.Deactivate` (`self.NS Active`)))))

(event `Triggered Event`
  ;[1 1 1] Event Code
  ;[0 0 0] Interaction event triggered
  ;;[0.005891 0.1406 0] True: Disables activator after a single usage
  ;;
  ;; False: Allows activator to be used more than once
  (if (`self.Single Use?`)
    ;;[0.005891 0.1406 0] Checks to see if this activator can be used more than once
    (`/Engine/EditorBlueprintResources/StandardMacros.DoOnce` false
      (:`Completed`
        _)))
  ;;[0.005891 0.1406 0] Play exposed sound
  (`GameplayStatics.PlaySound2D` (`self.Sound Selection`) 1.0 1.0 0.0 null null)
  ;;[0.005891 0.1406 0] Which event should the activator affect?
  (switch `/Game/Pickup/E_ActivationList` (`self.Activation List`)
    (:`NewEnumerator0`
      ;;[0.005891 0.1406 0] Checks to ensure each item in the arry is valid
      ;;
      ;; True: Activate the Popup Event for each item in the arry
      ;;
      ;; False: Do nothing
      (for (_array_element _array_index) (`self.Popup Actor`)
        (if (`KismetArrayLibrary.Array_IsValidIndex` (`self.Popup Actor`) _array_index)
          ;;[0.005891 0.1406 0] Tell the popup to do its actions, update it with the location of it's activator for the particle effect starting location
          (`/Game/CoreMechanics/Popup/BP_Popup_Base.Activate Play` _array_element (`SceneComponent.K2_GetComponentLocation` (`self.Activator Mesh`))))))))

(event `self.ReceiveActorBeginOverlap`
  (params (OtherActor :type "Actor Object Reference"))
  ;[1 0.3198 0.8863] Outline Collision
  (if (== OtherActor (`GameplayStatics.GetPlayerPawn` 0))
    (`MeshComponent.SetOverlayMaterial` (`self.Activator Mesh`) "/Game/Pickup/Activator_outline/Outline_Material.Outline_Material")))

(event `self.ReceiveActorEndOverlap`
  (params (OtherActor :type "Actor Object Reference"))
  ;[1 0.3198 0.8863] Outline Collision
  (if (== OtherActor (`GameplayStatics.GetPlayerPawn` 0))
    (`MeshComponent.SetOverlayMaterial` (`self.Activator Mesh`) null)))

(fn `IsInteractable`
  (returns (Interactable :type Boolean))
  (return (`self.Is Interactable?`)))

(fn `UserConstructionScript`)

(fn `What Can Activate Me?`
  (params (`Collided Component` :type "ActorComponent Object Reference"))
  (bind _collided_component (`self.Collided Component`))
  (bind _collided_component_2 (`self.Collided Component`))
  (set `self.Collided Component` `Collided Component`)
  ;[0.005891 0.1406 0] This gives the designer the option to select if this actor can be used by one, the other or both actors
  (switch `/Game/Pickup/E_ActorPickingUp` (`self.Who Can Activate Me?`)
    (:`NewEnumerator0`
      ;[0.005891 0.1406 0] Is the overlapping actor the player? (Check against the player's capsule component rather than the entire actor, so that other attached actors or children do not trigger the event)
      (if (or (== _collided_component_2 (`Character.CapsuleComponent` (`/Game/CoreMechanics/BP_Manager.Light Character` (`self.BP Manager`)))) (== _collided_component_2 (`Character.CapsuleComponent` (`/Game/CoreMechanics/BP_Manager.Dark Character` (`self.BP Manager`)))))
        ;[0.005891 0.1406 0] This controls if the rest of the code resumes, or stops due to not being the desired overlapping actor
        (set `self.Verified Actor` true :!label _label)
        (else
          (set `self.Verified Actor` false :!label _label_2)))
      (return))
    (:`NewEnumerator1`
      ;[0.005891 0.1406 0] Is the overlapping actor the assigned carry item? (Check against the static mesh component, so only one object triggers the event)
      (for _array_element (`self.CarryItem`)
        (if (== (`/Game/ThirdPerson/Blueprints/Item_Hold/BP_Carry_Item.StaticMesh` _array_element) (`self.Collided Component`))
          (goto _label)))
      (goto _label_2))
    (:`NewEnumerator2`
      ;[0.005891 0.1406 0] Is the overlapping actor the player (Check against the player's capsule component rather than the entire actor, so that other attached actors or children do not trigger the event) or the assigned carry item (Check against the static mesh component, so only one object triggers the event)
      (for _array_element_2 (`self.CarryItem`)
        (if (or (== (`/Game/ThirdPerson/Blueprints/Item_Hold/BP_Carry_Item.StaticMesh` _array_element_2) (`self.Collided Component`)) (== _collided_component (`Character.CapsuleComponent` (`/Game/CoreMechanics/BP_Manager.Light Character` (`self.BP Manager`)))) (== _collided_component (`Character.CapsuleComponent` (`/Game/CoreMechanics/BP_Manager.Dark Character` (`self.BP Manager`)))))
          (goto _label)
          (else
            (goto _label_2)))))))