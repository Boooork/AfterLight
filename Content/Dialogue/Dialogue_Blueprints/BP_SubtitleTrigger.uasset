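; Trigger actor that plays dialogue subtitles when the player character overlaps it.
; It creates a WBP_Subtitles widget from an exposed Data Table, starting at row "1", and has it calculate the dialogue's total time.
; An enum selects display in the viewport or on the actor's widget component for NPCs.
; An IsPlaying flag blocks retriggering until that time elapses; NPC mode then clears the component.
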(event `self.ReceiveActorBeginOverlap`
  (params (OtherActor :type "Actor Object Reference"))
  ;[0.005891 0.1406 0] True: The overlapping actor is the player character -AND- the dialogue is not already palying
  ;
  ; False: The dialogue is already playing
  (if (and (== OtherActor (`GameplayStatics.GetPlayerCharacter` 0)) (not (`self.IsPlaying?`)))
    (set `self.IsPlaying?` true)
    ;[0 0 0] Spawn the subtitle UI widget
    (bind _returnvalue (`|CreateWidget` "/Game/Dialogue/Subtitle_Widget/WBP_Subtitles.WBP_Subtitles_C" null (make `DataTableRowHandle` (`self.Data Table`) "1")))
    (bind _output_get (set `self.WBP Subtitles` _returnvalue))
    (`/Game/Dialogue/Subtitle_Widget/WBP_Subtitles.Calculate Total Time` _output_get (`self.Data Table`))
    (switch `/Game/Dialogue/Dialogue_Blueprints/Enum_Subtitles` (`self.Enum Subtitles`)
      (:`NewEnumerator0`
        (`UserWidget.AddToViewport` (`self.WBP Subtitles`) 0)
        ;[0.005891 0.1406 0] Wait the total time the dialogue is suppose to take, and then set Is Playing to false so the overlap can be retriggered and play the dialogue again
        (`KismetSystemLibrary.Delay` (`/Game/Dialogue/Subtitle_Widget/WBP_Subtitles.Total Time` (`self.WBP Subtitles`)))
        (set `self.IsPlaying?` false))
      (:`NewEnumerator1`
        (`WidgetComponent.SetWidget` (`self.Widget`) (`self.WBP Subtitles`))
        (`KismetSystemLibrary.Delay` (`/Game/Dialogue/Subtitle_Widget/WBP_Subtitles.Total Time` (`self.WBP Subtitles`)))
        (set `self.IsPlaying?` false)
        (`WidgetComponent.SetWidget` (`self.Widget`) null)
        (`KismetSystemLibrary.PrintString` "DONE")))
    (else
      (`KismetSystemLibrary.PrintString` "IsPLAYING ALREADY" true true (struct :`R` 1.0 :`G` 0.802997 :`A` 1.0)))))

(fn `UserConstructionScript`)