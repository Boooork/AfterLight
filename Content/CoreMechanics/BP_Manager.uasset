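; BP_Manager is the level manager for a light/dark character-swapping game, also handling checkpoint respawns, pausing, menu widgets, music and a directional level fade.
; Pressing E, when neither character is falling and swapping is allowed, possesses the other character with VFX, sound and camera shake.
; Each swap toggles post processors and the visibility and collision of "light" and "dark" tagged actors.
; Respawn uses the active character's checkpoint, restarting the level if none exists.
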(event `self.ReceiveBeginPlay`
  (bind _widget (`self.Widget`))
  (bind _widget_2 (`self.Widget`))
  (bind _widget_3 (`self.Widget`))
  (bind _widget_4 (`self.Widget`))
  (`self.Get All Tagged Light & Dark Actors`)
  (`self.Create Widgets`)
  ;[0 0 0] Starting Character Selection
  ;;[0.005891 0.1406 0] Does the game start with the player using the dark or light character. This is changed via the exposed variable inside of this BP
  (switch `/Game/ThirdPerson/Blueprints/E_StartingPlayer` (`self.Starting Character`)
    (:`NewEnumerator0`
      (`self.Swap (Light - Dark)`))
    (:`NewEnumerator1`
      (`self.Swap (Dark - Light)`)))
  ;;[0.005891 0.1406 0] Check to ensure there is a post processor set for light, dark and default
  (`self.Validate Post Processors`)
  ;[0.005891 0.1406 0] Play the sound you choose in the exposed variable slot of this BP
  (`GameplayStatics.PlaySound2D` (`self.Background Music`) 1.0 1.0 0.0 null null)
  ;[0 0 0] Level Transition (Faders)
  ;;[0.005891 0.1406 0] when the player completes the level, it will create the fadein/out and add start animating based off of the customizable direction
  (bind _returnvalue (`|CreateWidget` "/Game/UI/WBP_FadeinFadeout.WBP_FadeinFadeout_C" (`GameplayStatics.GetPlayerController` 0)))
  (set `self.Widget` _returnvalue)
  (`UserWidget.AddToViewport` _returnvalue 0)
  (switch `/Game/UI/E_FadeinFadeout` (`self.LevelFadeDirection`)
    (:`NewEnumerator0`
      ;;[0.005891 0.1406 0] the specific animation will play for the player going into the next level
      (`UserWidget.PlayAnimation` _widget_4 (`/Game/UI/WBP_FadeinFadeout.FadeinRight` _widget_4) 0.0 1 "Reverse" 1.0 false))
    (:`NewEnumerator1`
      (`UserWidget.PlayAnimation` _widget_3 (`/Game/UI/WBP_FadeinFadeout.FadeinLeft` _widget_3) 0.0 1 "Reverse" 1.0 false))
    (:`NewEnumerator2`
      (`UserWidget.PlayAnimation` _widget (`/Game/UI/WBP_FadeinFadeout.FadeinUp` _widget) 0.0 1 "Reverse" 1.0 false))
    (:`NewEnumerator3`
      (`UserWidget.PlayAnimation` _widget_2 (`/Game/UI/WBP_FadeinFadeout.FadeinDown` _widget_2) 0.0 1 "Reverse" 1.0 false))
    (:`NewEnumerator4`
      _))
  (`KismetSystemLibrary.Delay` 0.65)
  ;;[0.005891 0.1406 0] Enable inputs so that the "E" key can be used, otherise no inputs work
  (`self.EnableInput` (`GameplayStatics.GetPlayerController` 0)))

(event `Key|E`
  (params (Key :type "Key Structure"))
  ;[0 0 0] Swap Control Functionality
  (:`Pressed`
    (bind _isfalling (`self.Is Player Falling?`))
    (if (not _isfalling)
      ;;[0.005891 0.1406 0] Control if swap can or cannot occur
      (if (`self.Can Swap`)
        ;;[0.005891 0.1406 0] Set camera variable for camera shake later
        (bind _returnvalue (`GameplayStatics.GetActorOfClass` "/Game/ThirdPerson/Blueprints/BP_Camera.BP_Camera_C"))
        (set `self.Camera` (`/Game/ThirdPerson/Blueprints/BP_Camera.Camera` _returnvalue))
        ;;[0.005891 0.1406 0] Create Distortion widget so its ready for use
        (bind _returnvalue_2 (`|CreateWidget` "/Game/UI/Widgets/Distortion/WBP_Distortion.WBP_Distortion_C"))
        (set `self.WBP Distortion` _returnvalue_2)
        (`UserWidget.AddToViewport` (`self.WBP Distortion`) 0)
        ;;[0.005891 0.1406 0] This checks which character the player is currently using and how they swap to the other
        (switch `/Game/ThirdPerson/Blueprints/E_StartingPlayer` (`self.Starting Character`)
          (:`NewEnumerator0`
            (`self.Swap (Dark - Light)`)
            ;;[0.005891 0.1406 0] Depending on type of swap, these functions handle VFX and SFX
            (`self.Swap to Light - VFX/SFX`))
          (:`NewEnumerator1`
            (`self.Swap (Light - Dark)`)
            (`self.Swap to Dark - VFX/SFX`)))))))

(event `Respawn`
  ;[0 0 0] Respawn Functionality
  ;;[0.005891 0.1406 0] Which character is the player currently using?
  (switch `/Game/ThirdPerson/Blueprints/E_StartingPlayer` (`self.Starting Character`)
    (:`NewEnumerator0`
      ;;[0.005891 0.1406 0] This is so if the player "dies" before reaching a checkingout there is no "Access none" error. This checks if there is a checkpoint assigned via the exposed variable
      (`/Engine/EditorBlueprintResources/StandardMacros.IsValid` (`self.Check Point (Light)`)
        (:`Is Valid`
          ;;[0.005891 0.1406 0] Set the Light player's location and rotation to where the "RED ARROW" is located and pointing.
          (`self.K2_SetActorLocation` (`self.Light Character`) (`/Game/ThirdPerson/Blueprints/Checkpoints/BP_Checkpoint.Respawn Location` (`self.Check Point (Light)`)) false false)
          (`self.K2_SetActorRotation` (`self.Light Character`) (`/Game/ThirdPerson/Blueprints/Checkpoints/BP_Checkpoint.Respawn Rotation` (`self.Check Point (Light)`)) false))
        (:`Is Not Valid`
          ;;[0.005891 0.1406 0] Restart the level if the player "Dies" and there are no selected check points, this should only be possible if the player has never activated a checkpoint
          (bind _returnvalue (`GameplayStatics.GetCurrentLevelName` true :!label _label))
          (`GameplayStatics.OpenLevel` (`KismetStringLibrary.Conv_StringToName` _returnvalue))
          (`KismetSystemLibrary.PrintString` "LEVEL RESTARTED \nIf you would rather the player reset at a checkpoint then: \n \n1. Select BP_Manager in the world or in the outline panel \n2. Look for Check Point (Light) and Check Point (Dark) \n3. Use the eye dropper icon to select a starting check point for EACH \n" true true (struct :`R` 1.0 :`B` 0.070318 :`A` 1.0) 60.0))))
    (:`NewEnumerator1`
      (`/Engine/EditorBlueprintResources/StandardMacros.IsValid` (`self.Check Point (Dark)`)
        (:`Is Valid`
          ;;[0.005891 0.1406 0] Set the Dark player's location and rotation to where the "RED ARROW" is located and pointing.
          (`self.K2_SetActorLocation` (`self.Dark Character`) (`/Game/ThirdPerson/Blueprints/Checkpoints/BP_Checkpoint.Respawn Location` (`self.Check Point (Dark)`)) false false)
          (`self.K2_SetActorRotation` (`self.Dark Character`) (`/Game/ThirdPerson/Blueprints/Checkpoints/BP_Checkpoint.Respawn Rotation` (`self.Check Point (Dark)`)) false))
        (:`Is Not Valid`
          (goto _label))))))

(event `Key|P` :paused true
  (params (Key :type "Key Structure"))
  (:`Pressed`
    ;[0 0 0] Pause Functionality
    (if (`GameplayStatics.IsGamePaused`)
      (if (`self.On Unpause-able Menu?`)
        (`self.Unpause Fader`)
        ;;[0.005891 0.1406 0] delays the screen from being unpaused so the fader can play its length
        (`KismetSystemLibrary.Delay` 0.5)
        (`self.Return to Game`))
      (else
        (`self.Pause Game`)))))

(fn `Add Win / Lose Screen`
  (params (`Player Won?` :type Boolean))
  (`GameplayStatics.SetGamePaused` true)
  (set `/Game/UI/Widgets/Win_Lose/WBP_WinLose.Player Won?` `Player Won?` (`self.WBP Win/Lose`))
  (`UserWidget.AddToViewport` (`self.WBP Win/Lose`) 0))

(fn `Create Widgets`
  ;[0.005891 0.1406 0] Pause Screen
  (bind _returnvalue (`|CreateWidget` "/Game/UI/Widgets/Pause/WBP_Pause.WBP_Pause_C"))
  (set `self.WBP Pause Screen` _returnvalue)
  ;[0.005891 0.1406 0] Win /Lose Screen
  (bind _returnvalue_2 (`|CreateWidget` "/Game/UI/Widgets/Win_Lose/WBP_WinLose.WBP_WinLose_C"))
  (set `self.WBP Win/Lose` _returnvalue_2)
  ;[0.005891 0.1406 0] Confirmation Screen
  (bind _returnvalue_3 (`|CreateWidget` "/Game/UI/Widgets/Confirmation/WBP_ConfirmationScreen.WBP_ConfirmationScreen_C"))
  (set `self.WBP Confirmation Screen` _returnvalue_3)
  ;[0.005891 0.1406 0] Player HUD Screen
  (bind _returnvalue_4 (`|CreateWidget` "/Game/UI/Widgets/Player_HUD/WBP_PlayerHUD.WBP_PlayerHUD_C"))
  (set `self.WBP PlayerHUD` _returnvalue_4)
  ;[0.005891 0.1406 0] Main Menu Screen
  (bind _returnvalue_5 (`|CreateWidget` "/Game/UI/Widgets/Main_Menu/WBP_MainMenu.WBP_MainMenu_C"))
  (set `self.WBP MainMenu` _returnvalue_5)
  ;[0.005891 0.1406 0] Settings Screen
  (bind _returnvalue_6 (`|CreateWidget` "/Game/UI/Widgets/Settings/WBP_Settings.WBP_Settings_C"))
  (set `self.WBP Settings` _returnvalue_6))

(fn `Get All Tagged Light & Dark Actors`
  (bind _outactors (`GameplayStatics.GetAllActorsWithTag` "dark"))
  (set `self.Dark Actors (Tagged)` _outactors)
  (bind _outactors_2 (`GameplayStatics.GetAllActorsWithTag` "light"))
  (set `self.Light Actors (Tagged)` _outactors_2)
  (bind _outactors_3 (`GameplayStatics.GetAllActorsWithTag` "nc"))
  (set `self.Collide Actors` _outactors_3))

(fn `Is Player Falling?`
  (returns (IsFalling :type Boolean))
  (return (or (`NavMovementComponent.IsFalling` (`Character.CharacterMovement` (`self.Light Character`))) (`NavMovementComponent.IsFalling` (`Character.CharacterMovement` (`self.Dark Character`))))))

(fn `Pause Game`
  (set `self.On Unpause-able Menu?` true)
  (`GameplayStatics.SetGamePaused` true)
  (`UserWidget.AddToViewport` (`self.WBP Pause Screen`) 0))

(fn `Return to Game`
  (`Widget.RemoveFromParent` (`self.WBP Pause Screen`))
  (`WidgetBlueprintLibrary.SetInputMode_GameOnly` (`GameplayStatics.GetPlayerController` 0))
  (set `PlayerController.bShowMouseCursor` false (`GameplayStatics.GetPlayerController` 0))
  (`KismetSystemLibrary.PrintString` "REMOVED"))

(fn `Swap (Dark - Light)`
  ;[0 0 0] Swaps which character can be controlled and changes the world lighting through a camera like filter
  ;;[0.005891 0.1406 0] Sound Effect - Swap to dark (pitched down)
  (`GameplayStatics.PlaySound2D` "/Game/Sound/Player_Swap/Whoosh_Sub_15_Cue.Whoosh_Sub_15_Cue" 0.8 1.2 0.0 null null)
  ;;[0.005891 0.1406 0] Swap from the light character to the dark character
  (`Controller.Possess` (`GameplayStatics.GetPlayerController` 0) (`self.Dark Character`))
  ;;[0.005891 0.1406 0] Switch from the light processpr to the dark processor
  (set `self.Swapped` true)
  (set `PostProcessVolume.bEnabled` false (`self.PP_Light`))
  (set `PostProcessVolume.bEnabled` true (`self.PP_Dark`))
  ;;[0.005891 0.1406 0] Swap to the dark character
  (set `self.Starting Character` "NewEnumerator1")
  ;[0 0 0] Hide and reveal actors based on their tag, also controls their collision so they are passable
  ;;[0.005891 0.1406 0] Hide all tagged dark actors so they are invisible in the world and set their collision to false so they are collidable
  (for _array_element (`self.Light Actors (Tagged)`)
    (`self.SetActorHiddenInGame` _array_element true)
    (`self.SetActorEnableCollision` _array_element false)
    ;;[0.005891 0.1406 0] Show all tagged dark actors so they are visible in the world and set their collision to true so they are collidable
    (for _array_element_2 (`self.Dark Actors (Tagged)`)
      (`self.SetActorHiddenInGame` _array_element_2 false)
      (`self.SetActorEnableCollision` _array_element_2 true)
      ;;[0.005891 0.1406 0] Show the dark player and hide the light player
      (`self.SetActorHiddenInGame` (`self.Light Character`) true :!label _label)
      (`self.SetActorHiddenInGame` (`self.Dark Character`) false))
    (goto _label)))

(fn `Swap (Light - Dark)`
  ;[0 0 0] Swaps which character can be controlled and changes the world lighting through a camera like filter
  ;;[0.005891 0.1406 0] Sound Effect - Swap to dark (pitched up)
  (`GameplayStatics.PlaySound2D` "/Game/Sound/Player_Swap/Whoosh_Sub_15_Cue.Whoosh_Sub_15_Cue" 0.8 1.4 0.0 null null)
  ;;[0.005891 0.1406 0] Swap from the dark character to the light
  (`Controller.Possess` (`GameplayStatics.GetPlayerController` 0) (`self.Light Character`))
  ;;[0.005891 0.1406 0] Switch from the dark processor to the lighjt processor
  (set `self.Swapped` false)
  (set `PostProcessVolume.bEnabled` false (`self.PP_Dark`))
  (set `PostProcessVolume.bEnabled` true (`self.PP_Light`))
  ;;[0.005891 0.1406 0] Swap to the light character
  (set `self.Starting Character` "NewEnumerator0")
  ;[0 0 0] Hide and reveal actors based on their tag, also controls their collision so they are passable
  ;;[0.005891 0.1406 0] Show all tagged light actors so they are visible in the world and set their collision to true so they are collidable
  (for _array_element (`self.Light Actors (Tagged)`)
    (`self.SetActorHiddenInGame` _array_element false)
    (`self.SetActorEnableCollision` _array_element true)
    ;;[0.005891 0.1406 0] Hide all tagged dark actors so they are invisible in the world and set their collision to false so they are collidable
    (for _array_element_2 (`self.Dark Actors (Tagged)`)
      (`self.SetActorHiddenInGame` _array_element_2 true)
      (`self.SetActorEnableCollision` _array_element_2 false)
      ;;[0.005891 0.1406 0] Show the dark player and hide the light player
      (`self.SetActorHiddenInGame` (`self.Light Character`) false :!label _label)
      (`self.SetActorHiddenInGame` (`self.Dark Character`) true))
    (goto _label)))

(fn `Swap to Dark - VFX/SFX`
  (bind _wbp_distortion (`self.WBP Distortion`))
  (bind _returnvalue_location (`KismetMathLibrary.BreakTransform` (`self.GetTransform` (`self.Dark Character`))))
  (bind _returnvalue_location_2 (`KismetMathLibrary.BreakTransform` (`self.GetTransform` (`self.Light Character`))))
  (`NiagaraFunctionLibrary.SpawnSystemAtLocation` "/Game/SwapFX/NS_Light_Ring.NS_Light_Ring" _returnvalue_location_2)
  (`UserWidget.PlayAnimation` _wbp_distortion (`/Game/UI/Widgets/Distortion/WBP_Distortion.Distortion_Black_FadeIn` _wbp_distortion) 0.0 1 "Forward" 1.0 false)
  (`GameplayStatics.PlaySound2D` "/Game/SwapFX/Whoosh_Synth_30_Cue.Whoosh_Synth_30_Cue" 0.2 2.25 0.0 null null)
  (`NiagaraFunctionLibrary.SpawnSystemAtLocation` "/Game/SwapFX/NS_Distortion_Black.NS_Distortion_Black" _returnvalue_location)
  (`GameplayStatics.PlayWorldCameraShake` "/Game/SwapFX/BP_CameraShake.BP_CameraShake_C" (`SceneComponent.K2_GetComponentLocation` (`self.Camera`)) 0.0 1000.0))

(fn `Swap to Light - VFX/SFX`
  (bind _wbp_distortion (`self.WBP Distortion`))
  (bind _returnvalue_location (`KismetMathLibrary.BreakTransform` (`self.GetTransform` (`self.Dark Character`))))
  (bind _returnvalue_location_2 (`KismetMathLibrary.BreakTransform` (`self.GetTransform` (`self.Light Character`))))
  ;[0.005891 0.1406 0] Spawn a "NS_Ring" particle on the NEW characters location
  (`NiagaraFunctionLibrary.SpawnSystemAtLocation` "/Game/SwapFX/NS_BlackRing.NS_BlackRing" _returnvalue_location)
  ;[0.005891 0.1406 0] Plays a fade-in anim from Distortion widget based on the transition (light-->dark, dark-->light)
  (`UserWidget.PlayAnimation` _wbp_distortion (`/Game/UI/Widgets/Distortion/WBP_Distortion.Distortion_White_FadeIn_` _wbp_distortion) 0.0 1 "Forward" 1.0 false)
  ;[0.005891 0.1406 0] Sound effect based on type of transition (light vs dark)
  (`GameplayStatics.PlaySound2D` "/Game/SwapFX/Whoosh_Synth_30_Cue_Dark.Whoosh_Synth_30_Cue_Dark" 0.2 1.5 0.0 null null)
  ;[0.005891 0.1406 0] Spawn a "NS_Distortion" particle on the PREVIOUS character so it looks like they fade away
  (`NiagaraFunctionLibrary.SpawnSystemAtLocation` "/Game/SwapFX/NS_Distortion_Light.NS_Distortion_Light" _returnvalue_location_2)
  ;[0.005891 0.1406 0] Play BP_CameraShake
  (`GameplayStatics.PlayWorldCameraShake` "/Game/SwapFX/BP_CameraShake.BP_CameraShake_C" (`SceneComponent.K2_GetComponentLocation` (`self.Camera`)) 0.0 1000.0))

(fn `Unpause Fader`
  (bind _wbp_pause_screen (`self.WBP Pause Screen`))
  (`UserWidget.PlayAnimation` _wbp_pause_screen (`/Game/UI/Widgets/Pause/WBP_Pause.Background_Fade` _wbp_pause_screen) 0.0 1 "Reverse" 1.0 false)
  (`GameplayStatics.SetGamePaused` false))

(fn `UserConstructionScript`)

(fn `Validate Checkpoint`
  (`/Engine/EditorBlueprintResources/StandardMacros.IsValid` (`self.Check Point (Light)`)
    (:`Is Valid`
      (`/Engine/EditorBlueprintResources/StandardMacros.IsValid` (`self.Check Point (Dark)`)
        (:`Is Valid`
          (return))
        (:`Is Not Valid`
          _)))
    (:`Is Not Valid`
      _))
  (return))

(fn `Validate Post Processors`
  (`/Engine/EditorBlueprintResources/StandardMacros.IsValid` (`self.PP_Light`)
    (:`Is Valid`
      _)
    (:`Is Not Valid`
      (`KismetSystemLibrary.PrintString` "You did NOT select a Light  post processor! \n1. SELECT BP_Manager INSIDE OF THE WORLD \n2. LOOK FOR PP_LIGHT \n3. SELECT OPTION FOR PP_LIGHT" true true (struct :`R` 1.0 :`B` 0.054287 :`A` 1.0) 30.0)))
  (`/Engine/EditorBlueprintResources/StandardMacros.IsValid` (`self.PP_Dark`)
    (:`Is Valid`
      _)
    (:`Is Not Valid`
      (`KismetSystemLibrary.PrintString` "You did NOT select a Dark post processor! \n1. SELECT BP_Manager INSIDE OF THE WORLD \n2. LOOK FOR PP_DARK \n3. SELECT OPTION FOR PP_DARK" true true (struct :`R` 1.0 :`G` 0.068705 :`A` 1.0) 30.0)))
  (`/Engine/EditorBlueprintResources/StandardMacros.IsValid` (`self.PP_Default`)
    (:`Is Valid`
      _)
    (:`Is Not Valid`
      (`KismetSystemLibrary.PrintString` "You did NOT select a Default post processor! \n1. SELECT BP_Manager INSIDE OF THE WORLD \n2. LOOK FOR PP_DEFAULT \n3. SELECT OPTION FOR PP_DEFAULT" true true (struct :`R` 1.0 :`G` 0.068705 :`A` 1.0) 30.0)))
  (return))