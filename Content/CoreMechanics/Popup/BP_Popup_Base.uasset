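; Base popup actor that animates a pivot component's translation, rotation and scale by configurable per-axis offsets, each individually toggleable.
; BeginPlay caches the pivot's starting world transform, sets secondary mesh visibility and optionally plays forward.
; Three timelines lerp from start to offset values, with play rates derived from duration variables.
; ActivatePlay plays a sound and flip-flops between forward and reverse, while OnInteract only plays forward and IsInteractable returns false.
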(event `Activate Play`
  ;[1 1 1] Activate
  (`GameplayStatics.PlaySound2D` (`self.Sound Cue`) 1.0 1.0 0.0 null null)
  ;[0.005891 0.1406 0] Popup plays forward and then reverse, continously upon each activation
  (`/Engine/EditorBlueprintResources/StandardMacros.FlipFlop`
    (:`A`
      (`self.ActivateFoiward Play`))
    (:`B`
      (`self.Activate Reverse Play`))))

(event `self.ReceiveBeginPlay`
  ;[0 0 0] Begin Play
  ;;[0.005891 0.1406 0] Fill variables with current location, rotation and scale of actor
  (set `self.Starting World Location` (`SceneComponent.K2_GetComponentLocation` (`self.Pivot Point`)))
  (set `self.Starting World Rotation` (`SceneComponent.K2_GetComponentRotation` (`self.Pivot Point`)))
  (set `self.Starting World Scale` (`SceneComponent.K2_GetComponentScale` (`self.Pivot Point`)))
  ;;[0.005891 0.1406 0] Show secondary mesh in-world?
  (`SceneComponent.SetHiddenInGame` (`self.Secondary Mesh`) (not (`self.Show Secondary Mesh?`)) false)
  ;;[0.005891 0.1406 0] Should the popup animate when the game begins?
  (if (`self.Activate On Start?`)
    (`self.ActivateFoiward Play`)))

(event `ActivateFoiward Play`
  ;[0 0 0] Activate Popup (Add to any interaction event)
  ;;[0.005891 0.1406 0] True: Activate translate and then check for rotation and scale
  ;;
  ;; False: Do NOT translate and then check for rotation and scale
  (if (`self.Activate Translate`)
    (`self.Translate`))
  ;;[0.005891 0.1406 0] True: Activate rotate and then check for scale
  ;;
  ;; False: Do NOT rotate and then check for scale
  (if (`self.Activate Rotation`)
    (`self.Rotate`))
  ;;[0.005891 0.1406 0] True: Activate scale
  ;;
  ;; False: Do NOT scale
  (if (`self.Activate Scale?`)
    (`self.Scale`)))

(event `/Game/Pickup/BPI_Interactable.OnInteract`
  (params (InteractingPlayer :type "Character Object Reference"))
  ;[1 1 1] Activate (Remote)
  ;[0.005891 0.1406 0] When a remote (something) is activated with, run this code
  (`self.ActivateFoiward Play`))

(event `Activate Reverse Play`
  ;[1 1 1] Reverse Code
  ;[0.005891 0.1406 0] Play any currently enabled transform that is on a timeline in reverse
  (`self.Reverse Rotation`)
  (`self.Reverse Translation`)
  (`self.Reverse Scale`))

(event `Rotate`
  (bind (_starting_world_rotation_roll _starting_world_rotation_pitch _starting_world_rotation_yaw) (`KismetMathLibrary.BreakRotator` (`self.Starting World Rotation`)))
  ;[0 0 0] Rotation code
  ;;[0.005891 0.1406 0] Set the amount of time (SECONDS) it takes to animate
  (`TimelineComponent.SetPlayRate` (`self.Rotate Timeline`) (/ 1.0 (`self.Speed of Rotate`)))
  ;;[0.005891 0.1406 0] Get current rotation and add the exposed variables representing the axis(s) that you want to change. This is what allows the code to understand where you start and where your ending up
  (set `self.New Rotation` (`KismetMathLibrary.MakeRotator` (+ _starting_world_rotation_roll (`self.X-Axis (R) Amount`)) (+ _starting_world_rotation_pitch (`self.Y-Axis (R) Amount`)) (+ _starting_world_rotation_yaw (`self.Z-Axis (R) Amount`))))
  ;;[0.005891 0.1406 0] This time gives the base time and blend over time effect
  (bind (_direction _rotate_alpha) (`Timeline|Rotate Timeline` :!label _label)
    (:`Update`
      ;;[0.005891 0.1406 0] Take the updated blend value and set that value as the new world rotation
      (`SceneComponent.K2_SetWorldRotation` (`self.Pivot Point`) (`KismetMathLibrary.RLerp` (`self.Starting World Rotation`) (`self.New Rotation`) _rotate_alpha) false false))))

(event `Reverse Rotation`
  ;[0 0 0] Rotation code
  (goto _label :!via `Reverse`))

(event `Translate`
  (bind (_starting_world_location_x _starting_world_location_y _starting_world_location_z) (`KismetMathLibrary.BreakVector` (`self.Starting World Location`)))
  ;[0 0 0] Translate Code
  ;;[0.005891 0.1406 0] Set the amount of time (SECONDS) it takes to animate
  (`TimelineComponent.SetPlayRate` (`self.Translate Timeline`) (/ 1.0 (`self.Speed of Translate`)))
  ;;[0.005891 0.1406 0] Get current world location and add the exposed variables representing the axis(s) that you want to change. This is what allows the code to understand where you start and where your ending up
  (set `self.New Translate` (`KismetMathLibrary.MakeVector` (+ _starting_world_location_x (`self.X-Axis (T) Amount`)) (+ _starting_world_location_y (`self.Y-Axis (T) Amount`)) (+ _starting_world_location_z (`self.Z-Axis (T) Amount`))))
  ;;[0.005891 0.1406 0] This time gives the base time and blend over time effect
  (bind (_direction _translate_alpha) (`Timeline|Translate Timeline` :!label _label_2)
    (:`Update`
      ;;[0.005891 0.1406 0] Take the updated blend value and set that value as the new world location
      (`SceneComponent.K2_SetWorldLocation` (`self.Pivot Point`) (`KismetMathLibrary.VLerp` (`self.Starting World Location`) (`self.New Translate`) _translate_alpha) false false))))

(event `Reverse Translation`
  ;[0 0 0] Translate Code
  (goto _label_2 :!via `Reverse`))

(event `Scale`
  (bind (_starting_world_scale_x _starting_world_scale_y _starting_world_scale_z) (`KismetMathLibrary.BreakVector` (`self.Starting World Scale`)))
  ;[0 0 0] Scale Code
  ;;[0.005891 0.1406 0] Set the amount of time (SECONDS) it takes to animate
  (`TimelineComponent.SetPlayRate` (`self.Scale Timeline`) (/ 1.0 (`self.Speed of Scale`)))
  ;;[0.005891 0.1406 0] Get current world location and add the exposed variables representing the axis(s) that you want to change. This is what allows the code to understand where you start and where your ending up
  (set `self.New Scale` (`KismetMathLibrary.MakeVector` (+ _starting_world_scale_x (`self.X-Axis (S) Amount`)) (+ _starting_world_scale_y (`self.Y-Axis (S) Amount`)) (+ _starting_world_scale_z (`self.Z-Axis (S) Amount`))))
  ;;[0.005891 0.1406 0] This time gives the base time and blend over time effect
  (bind (_direction _scale_alpha) (`Timeline|Scale Timeline` :!label _label_3)
    (:`Update`
      ;;[0.005891 0.1406 0] Take the updated blend value and set that value as the new world location
      (`SceneComponent.SetWorldScale3D` (`self.Pivot Point`) (`KismetMathLibrary.VLerp` (`self.Starting World Scale`) (`self.New Scale`) _scale_alpha)))))

(event `Reverse Scale`
  ;[0 0 0] Scale Code
  (goto _label_3 :!via `Reverse`))

(fn `IsInteractable`
  (returns (Interactable :type Boolean))
  (return false))

(fn `UserConstructionScript`)