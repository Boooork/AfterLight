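; BP_SunMoon is an eclipse timer prop whose sun and moon are meant to converge, triggering the lose screen.
; Timelines rotate both roots and blend a directional light's color and intensity, during or after the countdown.
; CameraFollow tracks the player's Y or an assigned camera's Y and offset height.
; BeginPlay, Tick and ColorWorld are empty, leaving all that logic disconnected, including the only CameraFollow call.
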(event `self.ReceiveTick`
  (params (DeltaSeconds :type "Float (single-precision)")))

(event `self.ReceiveBeginPlay`)

(event `Color World`)

(event `Camera Follow`
  (bind _returnvalue_x (`KismetMathLibrary.BreakVector` (`self.K2_GetActorLocation`)))
  (bind (_returnvalue_x_2 _returnvalue_y _returnvalue_z) (`KismetMathLibrary.BreakVector` (`self.K2_GetActorLocation`)))
  (bind (_returnvalue_x_3 _returnvalue_y_2) (`KismetMathLibrary.BreakVector` (`self.K2_GetActorLocation` (`GameplayStatics.GetPlayerPawn` 0))))
  (bind (_returnvalue_x_4 _returnvalue_y_3 _returnvalue_z_2) (`KismetMathLibrary.BreakVector` (`self.K2_GetActorLocation` (`self.Player Camera`))))
  (switch `/Game/CoreMechanics/Time/Prop_Moon_Sun/E_FollowType` (`self.Follow Type`)
    (:`NewEnumerator0`
      ;[0 0 0] Sun and Moon Timer Follows Player
      ;;[0.005891 0.1406 0] Update actors left and right location (Y-Axis) with that of the player's
      (`self.K2_SetActorLocation` (`KismetMathLibrary.MakeVector` _returnvalue_x_2 _returnvalue_y_2 _returnvalue_z)))
    (:`NewEnumerator1`
      ;[0 0 0] Sun and Moon Timer Follows Camera
      ;;[0.005891 0.1406 0] Ensure there is a actor selected for player camera
      (`/Engine/EditorBlueprintResources/StandardMacros.IsValid` (`self.Player Camera`)
        (:`Is Valid`
          ;;[0.005891 0.1406 0] Update actors left and right location (Y-Axis) with that of the player's
          (`self.K2_SetActorLocation` (`KismetMathLibrary.MakeVector` _returnvalue_x _returnvalue_y_3 (+ _returnvalue_z_2 (`self.Height Value`)))))
        (:`Is Not Valid`
          (`KismetSystemLibrary.PrintString` "YOU FORGOT TO ASSIGN THE ECLIPSE TIMER A CAMERA \n1. CLICK ON ECLIPSE ACTOR IN-WORLD \n2. SELECT PLAYER CAMERA  \n3. USE EYE DROPPER" true true (struct :`R` 1.0 :`B` 0.03643 :`A` 1.0) 0.0))))))

(fn `UserConstructionScript`)